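; BP_Crabby is an enemy crab that chases the player, deals contact damage and dies when stomped.
; PawnSensing starts an AI move toward any BP_GIAMCharacter it sees.
; The DamageCapsule overlap applies damage when the character's own damage capsule also overlaps the crab.
; A falling character entering the HurtBox triggers a one-time stomp that bounces it upward, plays the death montage, then destroys the crab after a short delay.
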(event OnComponentBeginOverlap(DamageCapsule)
  (params (OverlappedComponent :type Primitive%20Component%20Object%20Reference) (OtherActor :type Actor%20Object%20Reference) (OtherComp :type Primitive%20Component%20Object%20Reference) (OtherBodyIndex :type Integer) (bFromSweep :type Boolean) (SweepResult :type Hit%20Result%20Structure%20%28by%20ref%29))
  (bind _self self)
  ;[1 1 1] Damage the player if they're in the damage zone
  (bind _asbp_giamcharacter (Utilities|Casting|CastToBP_GIAMCharacter OtherActor))
  (if (Collision|IsOverlappingActor (Variables|/Game/GIAMSystem/BP_GIAMCharacter.BP_GIAMCharacter_C|GetDamageCapsule _asbp_giamcharacter) _self :!class /Script/Engine.PrimitiveComponent)
    (Game|Damage|ApplyDamage _asbp_giamcharacter 1e+01 0 _self)))

(event OnSeePawn(PawnSensing)
  (params (Pawn :type Pawn%20Object%20Reference))
  ;[1 1 1] Crabby moves towards the player if they can see it
  (bind _asbp_giamcharacter (Utilities|Casting|CastToBP_GIAMCharacter Pawn))
  (AI|AIMoveTo self "0, 0, 0" _asbp_giamcharacter 5.0 false))

(event OnComponentBeginOverlap(HurtBox)
  (params (OverlappedComponent :type Primitive%20Component%20Object%20Reference) (OtherActor :type Actor%20Object%20Reference) (OtherComp :type Primitive%20Component%20Object%20Reference) (OtherBodyIndex :type Integer) (bFromSweep :type Boolean) (SweepResult :type Hit%20Result%20Structure%20%28by%20ref%29))
  ;[1 1 1] Once the player jumps on top of the crabby, destroy the actor
  (bind _asbp_giamcharacter (Utilities|Casting|CastToBP_GIAMCharacter OtherActor))
  (if (AI|Components|NavMovement|IsFalling (Variables|/Script/Engine.Character|GetCharacterMovement _asbp_giamcharacter))
    (Utilities|FlowControl|DoOnce false
      (:Completed
        (Character|LaunchCharacter _asbp_giamcharacter "0.000000,0.000000,700.000000" true true)
        (Animation|PlayAnimMontage "/Game/Assets/QuaterniusPlatformer/Enemies/FBX/AM_CrabDeath.AM_CrabDeath" 1.0 "None")
        (Utilities|FlowControl|Delay 0.7)
        (Actor|DestroyActor)))))

(event EventBeginPlay)

(event Collision|EventActorBeginOverlap
  (params (OtherActor :type Actor%20Object%20Reference)))

(event EventTick
  (params (DeltaSeconds :type Float%20%28single-precision%29)))

(fn ConstructionScript)