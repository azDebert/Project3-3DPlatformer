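; Boss enemy character that constantly chases the player using AI Move To on Tick, without pawn sensing.
; Entering DamageBox triggers the attack in ABP_Boss and disables movement and yaw rotation for a cooldown, while Box damages the player's overlapping DamageCapsule.
; Landing on AttackBox launches the player upward and removes boss health, gated by a timed DoOnce.
; At zero health, it plays a death montage, then destroys itself.
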(event OnComponentBeginOverlap(DamageBox)
  (params (OverlappedComponent :type Primitive%20Component%20Object%20Reference) (OtherActor :type Actor%20Object%20Reference) (OtherComp :type Primitive%20Component%20Object%20Reference) (OtherBodyIndex :type Integer) (bFromSweep :type Boolean) (SweepResult :type Hit%20Result%20Structure%20%28by%20ref%29))
  ;[1 1 1] Boss attack and its cooldown
  (Utilities|Casting|CastToBP_GIAMCharacter OtherActor)
  (bind _asabp_boss (Utilities|Casting|CastToABP_Boss (Components|SkeletalMesh|GetAnimInstance (Variables|Character|GetMesh))))
  (Variables|/Game/GIAMSystem/AI/ABP_Boss.ABP_Boss_C|SetBossAttack _asabp_boss true)
  (Components|Activation|SetActive (Variables|Character|GetCharacterMovement) false false)
  (Variables|Default|SetbUseControllerRotationYaw false)
  (Utilities|FlowControl|Delay 5.0)
  (CallFunction|StartMoving))

(event OnComponentBeginOverlap(Box)
  (params (OverlappedComponent :type Primitive%20Component%20Object%20Reference) (OtherActor :type Actor%20Object%20Reference) (OtherComp :type Primitive%20Component%20Object%20Reference) (OtherBodyIndex :type Integer) (bFromSweep :type Boolean) (SweepResult :type Hit%20Result%20Structure%20%28by%20ref%29))
  (bind _self self)
  ;[1 1 1] If the player is within the boss' bite zone then damage the player
  (bind _asbp_giamcharacter (Utilities|Casting|CastToBP_GIAMCharacter OtherActor))
  (if (Collision|IsOverlappingActor (Variables|/Game/GIAMSystem/BP_GIAMCharacter.BP_GIAMCharacter_C|GetDamageCapsule _asbp_giamcharacter) _self :!class /Script/Engine.PrimitiveComponent)
    (Game|Damage|ApplyDamage _asbp_giamcharacter 15.0 0 _self)))

(event OnComponentBeginOverlap(AttackBox)
  (params (OverlappedComponent :type Primitive%20Component%20Object%20Reference) (OtherActor :type Actor%20Object%20Reference) (OtherComp :type Primitive%20Component%20Object%20Reference) (OtherBodyIndex :type Integer) (bFromSweep :type Boolean) (SweepResult :type Hit%20Result%20Structure%20%28by%20ref%29))
  ;[1 1 1] Once the player jumps on top of the pad thats attached to the boss, damage him and if the boss' hp reaches 0 then destroy the actor
  (bind _asbp_giamcharacter (Utilities|Casting|CastToBP_GIAMCharacter OtherActor))
  (Utilities|FlowControl|DoOnce false :!label _label
    (:Completed
      (Character|LaunchCharacter _asbp_giamcharacter "0.000000,0.000000,700.000000" true true)
      (Variables|Default|SetHealth (- (Variables|Default|GetHealth) 1.0))
      (if (<= (Variables|Default|GetHealth) 0.0)
        (Animation|Montage|PlayMontage 0 "/Game/Assets/QuaterniusPlatformer/Enemies/FBX/AM_BossDeath.AM_BossDeath"
          (:then
            (Utilities|FlowControl|Delay 2.0)
            (Actor|DestroyActor)))
        (else
          (Utilities|FlowControl|Delay 2.0)
          (goto _label Reset))))))

(event Custom|StartMoving
  ;[1 1 1] After boss cooldown is over let it start moving
  (bind _asabp_boss (Utilities|Casting|CastToABP_Boss (Components|SkeletalMesh|GetAnimInstance (Variables|Character|GetMesh))))
  (Variables|/Game/GIAMSystem/AI/ABP_Boss.ABP_Boss_C|SetBossAttack _asabp_boss false)
  (Components|Activation|SetActive (Variables|Character|GetCharacterMovement) true false)
  (Variables|Default|SetbUseControllerRotationYaw true))

(event EventTick
  (params (DeltaSeconds :type Float%20%28single-precision%29))
  ;[1 1 1] No need for pawn sensing simple move to so it goes towards the player
  (bind _asbp_giamcharacter (Utilities|Casting|CastToBP_GIAMCharacter (Game|GetPlayerCharacter 0)))
  (AI|AIMoveTo self "0, 0, 0" _asbp_giamcharacter 5.0 false))

(event EventBeginPlay
  (Variables|Default|SetHealth (Variables|Default|GetMaxHealth)))

(fn ConstructionScript)