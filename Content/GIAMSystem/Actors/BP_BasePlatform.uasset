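; BP_BasePlatform is a base platform actor that reacts to BP_GIAMCharacter actors entering and leaving its overlap.
; On begin overlap, CheckOverlap searches OverlapActors, and an unlisted character is added and its index passed to ActivatePlatform, which destroys that character here.
; On end overlap, a listed character triggers DeactivatePlatform with a fixed zero index; that function is empty, and nothing removes entries from the array.
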(event EventBeginPlay)

(event Collision|EventActorBeginOverlap
  (params (OtherActor :type Actor%20Object%20Reference))
  ;[1 1 1] Add the player to the overlapping actors array and activate the platform if the player is touching the platform currently, then once the player is not in contact deactivate it
  (bind _asbp_giamcharacter (Utilities|Casting|CastToBP_GIAMCharacter OtherActor))
  (if (not (.IsOverlappingReturn (CallFunction|CheckOverlap _asbp_giamcharacter)))
    (bind _returnvalue (Utilities|Array|Add (Variables|Default|GetOverlap%20Actors) _asbp_giamcharacter))
    (CallFunction|ActivatePlatform _returnvalue)))

(event EventTick
  (params (DeltaSeconds :type Float%20%28single-precision%29)))

(event Collision|EventActorEndOverlap
  (params (OtherActor :type Actor%20Object%20Reference))
  ;[1 1 1] Add the player to the overlapping actors array and activate the platform if the player is touching the platform currently, then once the player is not in contact deactivate it
  (bind _asbp_giamcharacter (Utilities|Casting|CastToBP_GIAMCharacter OtherActor))
  (if (.IsOverlappingReturn (CallFunction|CheckOverlap _asbp_giamcharacter))
    (CallFunction|DeactivatePlatform)))

(fn ConstructionScript)

(fn CheckOverlap
  (params (OverlapActor :type BP%20GIAM%20Character%20Object%20Reference))
  ;[1 1 1] Check whether the overlapping actor is the player
  (for (_array_element _array_index) (Variables|Default|GetOverlap%20Actors)
    (if (== _array_element OverlapActor)
      (LocalVariables|SetisOverlapping true)
      (LocalVariables|SetTempIndex _array_index)))
  (if (LocalVariables|GetisOverlapping)
    (return true (LocalVariables|GetTempIndex))
    (else
      (return false -1))))

(fn ActivatePlatform
  (params (Index :type Integer))
  (Actor|DestroyActor (Utilities|Array|Get(acopy) (Variables|Default|GetOverlap%20Actors) Index)))

(fn DeactivatePlatform
  (params (Index :type Integer)))