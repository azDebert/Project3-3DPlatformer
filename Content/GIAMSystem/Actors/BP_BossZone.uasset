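; BP_BossZone is a trigger actor that shows and hides a boss health bar for the player's GIAM character.
; On begin overlap with player 0's BP_GIAMCharacter, it calls SpawnBossBar with its BossRef variable.
; On end overlap with that same character, it calls RemoveBossBar; other overlapping actors are ignored.
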(event EventBeginPlay)

(event Collision|EventActorBeginOverlap
  (params (OtherActor :type Actor%20Object%20Reference))
  (bind _asbp_giamcharacter (Utilities|Casting|CastToBP_GIAMCharacter (Game|GetPlayerCharacter 0)))
  (if (== _asbp_giamcharacter OtherActor)
    (Default|SpawnBossBar _asbp_giamcharacter (Variables|Default|GetBossRef))))

(event Collision|EventActorEndOverlap
  (params (OtherActor :type Actor%20Object%20Reference))
  (bind _asbp_giamcharacter (Utilities|Casting|CastToBP_GIAMCharacter (Game|GetPlayerCharacter 0)))
  (if (== _asbp_giamcharacter OtherActor)
    (Default|RemoveBossBar _asbp_giamcharacter)))

(fn ConstructionScript)