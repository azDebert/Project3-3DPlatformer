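; Gravity platform actor that changes an overlapping character's gravity scale and restores it after a delay.
; ActivatePlatform sets GravityScale on an OverlapActors entry, while begin overlap defers to the parent and this graph never calls ActivatePlatform itself.
; End overlap casts to BP_GIAMCharacter, gates on CheckOverlap, waits ZeroGravityDuration, then calls DeactivatePlatform on the first entry.
; DeactivatePlatform restores a hardcoded default gravity and removes that entry.
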(event EventBeginPlay
  (|CallParentFunction) ; This node is disabled and will not be called.\nDrag off pins to build functionality.
)

(event Collision|EventActorBeginOverlap
  (params (OtherActor :type Actor%20Object%20Reference))
  (|CallParentFunction OtherActor))

(event EventTick
  (params (DeltaSeconds :type Float%20%28single-precision%29))
  (|CallParentFunction DeltaSeconds) ; This node is disabled and will not be called.\nDrag off pins to build functionality.
)

(event Collision|EventActorEndOverlap
  (params (OtherActor :type Actor%20Object%20Reference))
  ;[1 1 1] Check if the player is still overlapping, if true then put a delay and deactivate the platform resetting the values
  (bind _asbp_giamcharacter (Utilities|Casting|CastToBP_GIAMCharacter OtherActor))
  (if (.IsOverlappingReturn (CallFunction|CheckOverlap _asbp_giamcharacter))
    (Utilities|FlowControl|Delay (Variables|Default|GetZeroGravityDuration))
    (CallFunction|DeactivatePlatform)))

(fn ConstructionScript
  (|CallParentFunction))

(fn ActivatePlatform
  (params (Index :type Integer))
  ;[1 1 1] Once player steps on, decrease their gravity
  (Variables|/Script/Engine.CharacterMovementComponent|SetGravityScale (Variables|/Script/Engine.Character|GetCharacterMovement (Utilities|Array|Get(acopy) (Variables|Default|GetOverlap%20Actors) Index)) (Variables|Default|GetGravity%20Scale)))

(fn DeactivatePlatform
  (params (Index :type Integer))
  ;[1 1 1] Reset gravity back to default
  (Variables|/Script/Engine.CharacterMovementComponent|SetGravityScale (Variables|/Script/Engine.Character|GetCharacterMovement (Utilities|Array|Get(acopy) (Variables|Default|GetOverlap%20Actors) Index)) 1.6)
  (Utilities|Array|RemoveIndex (Variables|Default|GetOverlap%20Actors) Index))