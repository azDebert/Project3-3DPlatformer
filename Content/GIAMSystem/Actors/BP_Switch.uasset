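; BP_Switch is an interactable lever that toggles a referenced fan.
; Interaction interface events highlight the mesh through custom depth on focus and call InteractOnServer on interact, which flips InteractToggle; a getter exposes the Widget.
; The InteractToggle RepNotify rotates the mesh between two orientations and calls FanSwitch on FanRef if valid, so the change follows replicated state.
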(event Custom|InteractOnServer
  (Variables|Default|SetInteractToggle (not (Variables|Default|GetInteractToggle))))

(event EventInterfaceToggleFocus
  (params (Focus :type Boolean))
  (Rendering|SetRenderCustomDepth (Variables|Default|GetStaticMesh) Focus))

(event EventBeginPlay
  (Rendering|SetRenderCustomDepth (Variables|Default|GetStaticMesh) false))

(event EventInterfaceInteract
  (CallFunction|InteractonServer))

(fn ConstructionScript)

(fn OnRepInteractToggle
  (bind _staticmesh (Variables|Default|GetStaticMesh))
  (bind _fanref (Variables|Default|GetFanRef))
  (bind _fanref_2 (Variables|Default|GetFanRef))
  (if (Variables|Default|GetInteractToggle)
    ;[1 1 1] Switch the lever, check if there is a reference to a Fan and then switch it on when interacted with the lever
    (Transformation|SetRelativeRotation _staticmesh "0.000000,180.000000,0.000000" false false)
    (Utilities|IsValid _fanref_2
      (:Is%20Valid
        (Default|FanSwitch _fanref_2)))
    (else
      (Transformation|SetRelativeRotation _staticmesh "0, 0, 0" false false)
      (Utilities|IsValid _fanref
        (:Is%20Valid
          (Default|FanSwitch _fanref))))))

(fn GetInteractionWidgetRef
  (return (Variables|Default|GetWidget)))