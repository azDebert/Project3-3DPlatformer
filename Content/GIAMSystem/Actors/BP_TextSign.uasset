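; BP_TextSign is a readable sign actor that shows a text prompt while the GIAM character is inside its box.
; Entering starts a looping timer that polls the character's Read flag while the prompt is visible.
; When the flag is set, it clears it, opens WBP_SignText with the sign's text, and switches to UI-only input with a cursor.
; Leaving only hides the prompt; the timer keeps running.
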(event OnComponentBeginOverlap(Box)
  (params (OverlappedComponent :type Primitive%20Component%20Object%20Reference) (OtherActor :type Actor%20Object%20Reference) (OtherComp :type Primitive%20Component%20Object%20Reference) (OtherBodyIndex :type Integer) (bFromSweep :type Boolean) (SweepResult :type Hit%20Result%20Structure%20%28by%20ref%29))
  ;[1 1 1] If the player steps into the zone, they are able to read the sign by pressing E
  (Utilities|Casting|CastToBP_GIAMCharacter OtherActor)
  (Rendering|SetVisibility (Variables|Default|GetTextRender) true false)
  (Utilities|Time|SetTimerbyEvent (delegate Custom|ReadText) 0.1 true))

(event OnComponentEndOverlap(Box)
  (params (OverlappedComponent :type Primitive%20Component%20Object%20Reference) (OtherActor :type Actor%20Object%20Reference) (OtherComp :type Primitive%20Component%20Object%20Reference) (OtherBodyIndex :type Integer))
  ;[1 1 1] If the player steps into the zone, they are able to read the sign by pressing E
  (Utilities|Casting|CastToBP_GIAMCharacter OtherActor)
  (Rendering|SetVisibility (Variables|Default|GetTextRender) false false))

(event Custom|ReadText
  (bind _returnvalue (Game|GetPlayerController 0))
  ;[1 1 1] If the player steps into the zone, they are able to read the sign by pressing E
  (if (Rendering|IsVisible (Variables|Default|GetTextRender))
    (bind _asbp_giamcharacter (Utilities|Casting|CastToBP_GIAMCharacter (Game|GetPlayerCharacter 0)))
    (if (Variables|/Game/GIAMSystem/BP_GIAMCharacter.BP_GIAMCharacter_C|GetRead _asbp_giamcharacter)
      (Variables|/Game/GIAMSystem/BP_GIAMCharacter.BP_GIAMCharacter_C|SetRead _asbp_giamcharacter false)
      (bind _returnvalue_2 (UserInterface|CreateWidget "/Game/GIAMSystem/WidgetBPs/WBP_SignText.WBP_SignText_C"))
      (UserInterface|Viewport|AddtoViewport _returnvalue_2 0)
      (Variables|/Game/GIAMSystem/WidgetBPs/WBP_SignText.WBP_SignText_C|SetSignText _returnvalue_2 (Variables|Default|GetSign%20Text))
      (Variables|/Script/Engine.PlayerController|SetbShowMouseCursor _returnvalue true)
      (Input|SetInputModeUIOnly _returnvalue 0 "DoNotLock" false))))

(event EventBeginPlay)

(event Collision|EventActorBeginOverlap
  (params (OtherActor :type Actor%20Object%20Reference)))

(event EventTick
  (params (DeltaSeconds :type Float%20%28single-precision%29)))

(fn ConstructionScript)