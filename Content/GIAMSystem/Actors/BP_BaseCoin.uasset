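; BP_BaseCoin is a coin pickup that adds coins to the character that collects it and persists the total.
; On pickup it loads the BPSG_GameSave in slot "1", adds CoinsToAdd to the character's Coins, writes that total to PlayerCoins and saves synchronously.
; If the save cast fails, neither the coin increment nor the parent OnPickup runs.
; Pickup eligibility is left entirely to the parent class.
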(event EventBeginPlay
  (|CallParentFunction) ; This node is disabled and will not be called.\nDrag off pins to build functionality.
)

(event Collision|EventActorBeginOverlap
  (params (OtherActor :type Actor%20Object%20Reference))
  (|CallParentFunction OtherActor) ; This node is disabled and will not be called.\nDrag off pins to build functionality.
)

(event EventTick
  (params (DeltaSeconds :type Float%20%28single-precision%29))
  (|CallParentFunction DeltaSeconds) ; This node is disabled and will not be called.\nDrag off pins to build functionality.
)

(event EventOnPickup
  (params (Character :type BP%20GIAM%20Character%20Object%20Reference))
  ;[1 1 1] Load game save once the player picks up a coin, set the current player coins once he picks up another one in a new level then save game again
  (bind _returnvalue (SaveGame|LoadGamefromSlot "1"))
  (bind _asbpsg_game_save (Utilities|Casting|CastToBPSG_GameSave _returnvalue))
  (bind _output_get (Variables|/Script/GIAM.GIAMCharacter|SetCoins Character (+ (Variables|/Script/GIAM.GIAMCharacter|GetCoins Character) (Variables|Default|GetCoinsToAdd))))
  (Variables|/Game/GIAMSystem/BPSG_GameSave.BPSG_GameSave_C|SetPlayerCoins _asbpsg_game_save _output_get)
  (SaveGame|SaveGametoSlot _asbpsg_game_save "1")
  (|CallParentFunction Character))

(fn ConstructionScript
  (|CallParentFunction))

(fn CanbePickedUp
  (params (Character :type BP%20GIAM%20Character%20Object%20Reference))
  (bind _canbepickedup (|CallParentFunction Character))
  (return _canbepickedup))