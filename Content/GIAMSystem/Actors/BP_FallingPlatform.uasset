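; BP_FallingPlatform is a platform that falls after a BP_GIAMCharacter steps on it, then respawns.
; The first overlap with its Box swaps the mesh materials to red as a warning, then enables physics on the mesh after a short delay.
; After a further delay the actor destroys itself and spawns a new copy at the mesh location saved on BeginPlay, without carrying over rotation or scale.
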(event OnComponentBeginOverlap(Box)
  (params (OverlappedComponent :type Primitive%20Component%20Object%20Reference) (OtherActor :type Actor%20Object%20Reference) (OtherComp :type Primitive%20Component%20Object%20Reference) (OtherBodyIndex :type Integer) (bFromSweep :type Boolean) (SweepResult :type Hit%20Result%20Structure%20%28by%20ref%29))
  ;[1 1 1] Get the original location of the platform, change the material once player steps on, delay then simulate physics so the platform falls, another delay then destroy the previous platform and respawn it
  (Utilities|Casting|CastToBP_GIAMCharacter OtherActor)
  (Utilities|FlowControl|DoOnce false
    (:Completed
      (Rendering|Material|SetMaterial (Variables|Default|GetStaticMesh) 0 "/Game/Assets/QuaterniusPlatformer/Cubes/FBX/Red_Dark.Red_Dark")
      (Rendering|Material|SetMaterial (Variables|Default|GetStaticMesh) 1 "/Game/Assets/QuaterniusPlatformer/Cubes/FBX/Red.Red")
      (Utilities|FlowControl|Delay 1.0)
      (Physics|SetSimulatePhysics (Variables|Default|GetStaticMesh) true)
      (Utilities|FlowControl|Delay 4.0)
      (Actor|DestroyActor)
      (Game|SpawnActorfromClass "BP_FallingPlatform_C" (Math|Conversions|ToTransform(Vector) (Variables|Default|GetLocationOriginal)) "Undefined" "MultiplyWithRoot" 0 0))))

(event EventBeginPlay
  ;[1 1 1] Get the original location of the platform, change the material once player steps on, delay then simulate physics so the platform falls, another delay then destroy the previous platform and respawn it
  (Variables|Default|SetLocationOriginal (Transformation|GetWorldLocation (Variables|Default|GetStaticMesh))))

(fn ConstructionScript)