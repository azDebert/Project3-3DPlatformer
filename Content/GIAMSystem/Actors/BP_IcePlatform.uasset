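; Ice platform actor that makes characters slide by altering their movement settings.
; ActivatePlatform lowers ground friction, acceleration and walking braking on the indexed OverlapActors entry.
; DeactivatePlatform restores hardcoded defaults on element 0, regardless of the index passed, then removes the given index from the array.
; The event graph holds only disabled stubs, so nothing in this graph calls either function.
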(event EventBeginPlay
  (|CallParentFunction) ; This node is disabled and will not be called.\nDrag off pins to build functionality.
)

(event Collision|EventActorBeginOverlap
  (params (OtherActor :type Actor%20Object%20Reference))
  (|CallParentFunction OtherActor) ; This node is disabled and will not be called.\nDrag off pins to build functionality.
)

(event EventTick
  (params (DeltaSeconds :type Float%20%28single-precision%29))
  (|CallParentFunction DeltaSeconds) ; This node is disabled and will not be called.\nDrag off pins to build functionality.
)

(fn ConstructionScript
  (|CallParentFunction))

(fn ActivatePlatform
  (params (Index :type Integer))
  (bind _overlap_actors (Variables|Default|GetOverlap%20Actors))
  (bind _output (Utilities|Array|Get(acopy) _overlap_actors Index))
  (bind _charactermovement (Variables|/Script/Engine.Character|GetCharacterMovement _output))
  ;[1 1 1] Set Ice values
  (Variables|/Script/Engine.CharacterMovementComponent|SetGroundFriction _charactermovement 0.4)
  (Variables|/Script/Engine.CharacterMovementComponent|SetMaxAcceleration _charactermovement 4e+02)
  (Variables|/Script/Engine.CharacterMovementComponent|SetBrakingDecelerationWalking _charactermovement 1e+02))

(fn DeactivatePlatform
  (params (Index :type Integer))
  (bind _overlap_actors (Variables|Default|GetOverlap%20Actors))
  (bind _output (Utilities|Array|Get(acopy) _overlap_actors))
  (bind _charactermovement (Variables|/Script/Engine.Character|GetCharacterMovement _output))
  ;[1 1 1] Reset values to default
  (Variables|/Script/Engine.CharacterMovementComponent|SetGroundFriction _charactermovement 8.0)
  (Variables|/Script/Engine.CharacterMovementComponent|SetMaxAcceleration _charactermovement 1.5e+03)
  (Variables|/Script/Engine.CharacterMovementComponent|SetBrakingDecelerationWalking _charactermovement 2e+03)
  (Utilities|Array|RemoveIndex (Variables|Default|GetOverlap%20Actors) Index))