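; BP_MapPortal is a level portal actor that sends the player to another map when they walk into it.
; On BeginPlay it applies an overlay material to its mesh to tell portals apart and shows the target level name on a text render.
; When a BP_GIAMCharacter overlaps its box, it plays a bubbles sound, waits briefly, then opens the named level.
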(event OnComponentBeginOverlap(Box)
  (params (OverlappedComponent :type Primitive%20Component%20Object%20Reference) (OtherActor :type Actor%20Object%20Reference) (OtherComp :type Primitive%20Component%20Object%20Reference) (OtherBodyIndex :type Integer) (bFromSweep :type Boolean) (SweepResult :type Hit%20Result%20Structure%20%28by%20ref%29))
  ;[1 1 1] When player walks into the zone, there is a sound played then they get teleported to the next level. The name of the level is displayed above the portal
  (Utilities|Casting|CastToBP_GIAMCharacter OtherActor)
  (Audio|PlaySound2D "/Game/Assets/Ultimate_Platformer_Asset_Pack/Bonus_SFX_Pack/bubbles-sound.bubbles-sound" 1.0 1.0 0.0 0 0)
  (Utilities|FlowControl|Delay 1.0)
  (Game|OpenLevel(byName) (Variables|Default|GetLevel%20Name)))

(event Collision|EventActorBeginOverlap
  (params (OtherActor :type Actor%20Object%20Reference)))

(event EventTick
  (params (DeltaSeconds :type Float%20%28single-precision%29)))

(event EventBeginPlay
  ;[1 1 1] Set portal material overlay to differentiate them
  (Rendering|Material|SetOverlayMaterial (Variables|Default|GetStaticMesh) (Variables|Default|GetNew%20Overlay%20Material) :!class /Script/Engine.MeshComponent)
  ;[1 1 1] When player walks into the zone, there is a sound played then they get teleported to the next level. The name of the level is displayed above the portal
  (Rendering|Components|TextRender|SetText (Variables|Default|GetTextRender) (Utilities|Text|ToText(Name) (Variables|Default|GetLevel%20Name))))

(fn ConstructionScript)