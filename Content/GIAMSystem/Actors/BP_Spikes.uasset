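; BP_Spikes is a spike hazard that hurts the player character and bounces it upward.
; Its ActivatePlatform function takes an index into OverlapActors, casts that actor to BP_GIAMCharacter, then applies fixed damage and a vertical launch that overrides current velocity.
; The handled entry is then removed from the array if still valid.
; The event graph holds only disabled stubs, so nothing here triggers the function.
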(event EventBeginPlay
  (|CallParentFunction) ; This node is disabled and will not be called.\nDrag off pins to build functionality.
)

(event Collision|EventActorBeginOverlap
  (params (OtherActor :type Actor%20Object%20Reference))
  (|CallParentFunction OtherActor) ; This node is disabled and will not be called.\nDrag off pins to build functionality.
)

(event EventTick
  (params (DeltaSeconds :type Float%20%28single-precision%29))
  (|CallParentFunction DeltaSeconds) ; This node is disabled and will not be called.\nDrag off pins to build functionality.
)

(fn ConstructionScript
  (|CallParentFunction))

(fn ActivatePlatform
  (params (Index :type Integer))
  ;[1 1 1] Damage the player and launch them upwards
  (bind _asbp_giamcharacter (Utilities|Casting|CastToBP_GIAMCharacter (Utilities|Array|Get(acopy) (Variables|Default|GetOverlap%20Actors) Index)))
  (Game|Damage|ApplyDamage _asbp_giamcharacter 5.0 0 self)
  (Character|LaunchCharacter _asbp_giamcharacter (Math|Vector|MakeVector 0.0 0.0 7.5e+02) true true)
  (Utilities|IsValid (Utilities|Array|Get(acopy) (Variables|Default|GetOverlap%20Actors) Index)
    (:Is%20Valid
      (Utilities|Array|RemoveIndex (Variables|Default|GetOverlap%20Actors) Index))))