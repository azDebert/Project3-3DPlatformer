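; BP_BaseHealth is a base health pickup that restores a character's health.
; On pickup it adds HealthToAdd to the character's Health, clamped between zero and MaxHealth, then calls the parent pickup logic.
; CanBePickedUp overrides the parent check, refusing pickup when the character's Health already equals MaxHealth.
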(event EventBeginPlay
  (|CallParentFunction) ; This node is disabled and will not be called.\nDrag off pins to build functionality.
)

(event Collision|EventActorBeginOverlap
  (params (OtherActor :type Actor%20Object%20Reference))
  (|CallParentFunction OtherActor) ; This node is disabled and will not be called.\nDrag off pins to build functionality.
)

(event EventTick
  (params (DeltaSeconds :type Float%20%28single-precision%29))
  (|CallParentFunction DeltaSeconds) ; This node is disabled and will not be called.\nDrag off pins to build functionality.
)

(event EventOnPickup
  (params (Character :type BP%20GIAM%20Character%20Object%20Reference))
  (Variables|/Script/GIAM.GIAMCharacter|SetHealth Character (Math|Float|Clamp(Float) (+ (Variables|/Script/GIAM.GIAMCharacter|GetHealth Character) (Variables|Default|GetHealthToAdd)) 0.0 (Variables|/Script/GIAM.GIAMCharacter|GetMaxHealth Character)))
  (|CallParentFunction Character))

(fn ConstructionScript
  (|CallParentFunction))

(fn CanbePickedUp
  (params (Character :type BP%20GIAM%20Character%20Object%20Reference))
  ;[1 1 1] Check if the health is below max health, if so then the player is able to pick up health
  (|CallParentFunction Character)
  (if (== (Variables|/Script/GIAM.GIAMCharacter|GetMaxHealth Character) (Variables|/Script/GIAM.GIAMCharacter|GetHealth Character))
    (return false)
    (else
      (return true))))