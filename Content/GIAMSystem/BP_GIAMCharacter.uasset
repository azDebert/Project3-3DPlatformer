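; Player character for a platformer, handling double-jump feedback, cooldown dash, ledge hanging, interaction, camera zoom and HUD, pause, boss bar and win widgets.
; While falling, Tick runs two line traces to snap onto ledges and zero gravity until jump restores it.
; Damage applies knockback and mesh flicker; death reloads the level, while R respawns a fresh character at the checkpoint transform.
; BeginPlay loads saved coins and enables the interaction trace component.
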(event Custom|Fall%20Death
  ;[1 1 1] Check If the player has reached 0 HP, if so then destroy him and respawn, if false then set up a visibility switch to "animate" damage
  (Pawn|Components|CharacterMovement|DisableMovement (Variables|Character|GetCharacterMovement))
  (Utilities|FlowControl|Delay 2.0)
  (Actor|DestroyActor)
  (bind _returnvalue (Game|GetCurrentLevelName true))
  (Game|OpenLevel(byName) (Utilities|String|StringToName _returnvalue)))

(event Custom|SpawnBossBar
  (params (BossRef :type BP%20Boss%20Object%20Reference))
  ;[1 1 1] Spawn boss bar when player enters boss zone, remove it once the boss is dead or player leaves boss zone
  (Utilities|IsValid BossRef
    (:Is%20Valid
      (bind _returnvalue (UserInterface|CreateWidget "/Game/GIAMSystem/WidgetBPs/WBP_BossBar.WBP_BossBar_C" 0 BossRef))
      (bind _output_get (Variables|Default|SetBossBarRef _returnvalue))
      (UserInterface|Viewport|AddtoViewport _output_get 0))))

(event Custom|RemoveBossBar
  ;[1 1 1] Spawn boss bar when player enters boss zone, remove it once the boss is dead or player leaves boss zone
  (Utilities|IsValid (Variables|Default|GetBossBarRef)
    (:Is%20Valid
      (Widget|RemovefromParent (Variables|Default|GetBossBarRef)))))

(event Input|EnhancedActionEvents|EnhancedInputActionIA_Jump
  (params (ActionValue :type Boolean) (ElapsedSeconds :type Float%20%28double-precision%29) (TriggeredSeconds :type Float%20%28double-precision%29) (InputAction :type Input%20Action%20Object%20Reference :default "/Game/GIAMSystem/Input/Actions/IA_Jump.IA_Jump"))
  (bind _charactermovement (Variables|Character|GetCharacterMovement))
  ;[1 1 1] Jumping bool for ABP
  (:Triggered
    (if (Variables|Default|GetbCanMove)
      ;[1 1 1] Reset variables after hanging
      (if ActionValue
        (Character|Jump :!label _label)
        (Variables|Default|SetJumping true))
      (else
        (Variables|/Script/Engine.CharacterMovementComponent|SetGravityScale _charactermovement (Variables|Default|GetTemporaryGravity))
        (Variables|Default|SetbCanMove true)
        (Variables|/Script/Engine.MovementComponent|SetVelocity _charactermovement (Math|Vector|MakeVector 0.0 0.0 (Variables|/Script/Engine.CharacterMovementComponent|GetJumpZVelocity _charactermovement)))
        (goto _label))))
  (:Completed
    (Variables|Default|SetJumping false)))

(event Input|EnhancedActionEvents|EnhancedInputActionIA_Pause
  (params (ActionValue :type Boolean) (ElapsedSeconds :type Float%20%28double-precision%29) (TriggeredSeconds :type Float%20%28double-precision%29) (InputAction :type Input%20Action%20Object%20Reference :default "/Game/GIAMSystem/Input/Actions/IA_Pause.IA_Pause"))
  (bind _returnvalue (Game|GetPlayerController 0))
  ;[1 1 1] Pause menu
  (:Started
    (bind _returnvalue_2 (UserInterface|CreateWidget "/Game/GIAMSystem/WidgetBPs/WBP_Pause.WBP_Pause_C"))
    (UserInterface|Viewport|AddtoViewport _returnvalue_2 0)
    (Variables|/Script/Engine.PlayerController|SetbShowMouseCursor _returnvalue true)
    (Input|SetInputModeUIOnly _returnvalue 0 "DoNotLock" false)
    (Game|SetGamePaused true)))

(event Input|EnhancedActionEvents|EnhancedInputActionIA_Interact
  (params (ActionValue :type Boolean) (ElapsedSeconds :type Float%20%28double-precision%29) (TriggeredSeconds :type Float%20%28double-precision%29) (InputAction :type Input%20Action%20Object%20Reference :default "/Game/GIAMSystem/Input/Actions/IA_Interact.IA_Interact"))
  (bind _ac_interactiontrace (Variables|Default|GetAC_InteractionTrace))
  ;[1 1 1] Interaction
  (:Triggered
    (Default|TrytoInteract _ac_interactiontrace true))
  (:Completed
    (Default|TrytoInteract _ac_interactiontrace false)))

(event Input|EnhancedActionEvents|EnhancedInputActionIA_Dash
  (params (ActionValue :type Boolean) (ElapsedSeconds :type Float%20%28double-precision%29) (TriggeredSeconds :type Float%20%28double-precision%29) (InputAction :type Input%20Action%20Object%20Reference :default "/Game/GIAMSystem/Input/Actions/IA_Dash.IA_Dash"))
  (bind _returnvalue (Transformation|GetVelocity))
  (bind _returnvalue_2 (* _returnvalue 6.0))
  ;[1 1 1] Dash with cooldown, effect and sound
  (if (not (Variables|Default|GetisDashing))
    (Variables|Default|SetisDashing true)
    (Character|LaunchCharacter (Math|Vector|MakeVector (.x _returnvalue_2) (.y _returnvalue_2) 0.0) false false)
    (Niagara|SpawnSystemAttached "/Game/GIAMSystem/Niagara/NS_Dash.NS_Dash" (Variables|Default|GetOtherEffects) "None" "0, 0, 0" "0, 0, 0" "KeepRelativeOffset" false)
    (Audio|PlaySoundatLocation "/Game/Assets/Ultimate_Platformer_Asset_Pack/Bonus_SFX_Pack/jump-sound-3.jump-sound-3" "0, 0, 0" "0, 0, 0" 0.5 1.0 0.0 0 0 0 0)
    (Utilities|FlowControl|Delay 2.0)
    (Variables|Default|SetisDashing false)))

(event Input|EnhancedActionEvents|EnhancedInputActionIA_ReadSign
  (params (ActionValue :type Boolean) (ElapsedSeconds :type Float%20%28double-precision%29) (TriggeredSeconds :type Float%20%28double-precision%29) (InputAction :type Input%20Action%20Object%20Reference :default "/Game/GIAMSystem/Input/Actions/IA_ReadSign.IA_ReadSign"))
  ;[1 1 1] Read Sign
  (:Started
    (Variables|Default|SetRead true)
    (Utilities|FlowControl|Delay 0.1)
    (Variables|Default|SetRead false)))

(event EventOnLanded
  (params (Hit :type Hit%20Result%20Structure%20%28by%20ref%29))
  ;[1 1 1] Reset jump Count
  (Variables|Default|SetJumpCount 0))

(event Game|Damage|EventAnyDamage
  (params (Damage :type Float%20%28single-precision%29) (DamageType :type Damage%20Type%20Object%20Reference) (InstigatedBy :type Controller%20Object%20Reference) (DamageCauser :type Actor%20Object%20Reference))
  (bind _returnvalue (Transformation|GetActorLocation DamageCauser))
  (bind _returnvalue_2 (Transformation|GetActorLocation))
  (bind _returnvalue_3 (- _returnvalue _returnvalue_2))
  (bind _returnvalue_4 (* _returnvalue_3 -15.0))
  ;[1 1 1] Receiving Damage
  (Character|LaunchCharacter (Math|Vector|MakeVector (.x _returnvalue_4) (.y _returnvalue_4) 4e+01) false true)
  (Variables|Default|SetHealth (- (Variables|Default|GetHealth) Damage))
  ;[1 1 1] Check If the player has reached 0 HP, if so then destroy him and respawn, if false then set up a visibility switch to "animate" damage
  (if (== (Variables|Default|GetHealth) 0.0)
    (Utilities|FlowControl|Delay 0.5)
    (Variables|Default|SetbIsDead true)
    (Pawn|Components|CharacterMovement|DisableMovement (Variables|Character|GetCharacterMovement))
    (Utilities|FlowControl|Delay 2.0)
    (Actor|DestroyActor)
    (bind _returnvalue_5 (Game|GetCurrentLevelName true))
    (Game|OpenLevel(byName) (Utilities|String|StringToName _returnvalue_5))
    (else
      (Collision|SetCollisionEnabled (Variables|Default|GetDamageCapsule) "NoCollision")
      (Rendering|SetVisibility (Variables|Character|GetMesh) false false)
      (Utilities|FlowControl|Delay 0.1)
      (Rendering|SetVisibility (Variables|Character|GetMesh) true false)
      (Utilities|FlowControl|Delay 0.1)
      (Rendering|SetVisibility (Variables|Character|GetMesh) false false)
      (Utilities|FlowControl|Delay 0.1)
      (Rendering|SetVisibility (Variables|Character|GetMesh) true false)
      (Utilities|FlowControl|Delay 0.1)
      (Collision|SetCollisionEnabled (Variables|Default|GetDamageCapsule) "QueryAndPhysics"))))

(event EventTick
  (params (DeltaSeconds :type Float%20%28single-precision%29))
  (bind _returnvalue (Transformation|GetActorLocation))
  (bind _returnvalue_2 (Transformation|GetActorForwardVector))
  (bind _returnvalue_3 (Transformation|GetActorLocation))
  (bind _charactermovement (Variables|Character|GetCharacterMovement))
  (bind _returnvalue_4 (* _returnvalue_2 75.0))
  (bind _returnvalue_5 (+ _returnvalue _returnvalue_4))
  (if (Variables|Default|GetbWinCondition)
    (Utilities|FlowControl|DoOnce false
      (:Completed
        (bind _returnvalue_6 (UserInterface|CreateWidget "/Game/GIAMSystem/WidgetBPs/WBP_WinScreen.WBP_WinScreen_C"))
        (UserInterface|Viewport|AddtoViewport _returnvalue_6 0)
        (Variables|/Script/Engine.PlayerController|SetbShowMouseCursor (Game|GetPlayerController 0) true)
        (Input|SetInputModeUIOnly 0 0 "DoNotLock" false)))
    (else
      ;[1 1 1] Check if player is dead to update anim
      (bind _output_get (Variables|Default|SetbIsDead (<= (Variables|Default|GetHealth) 0.0)))
      (if (not _output_get)
        ;[1 1 1] Check if player is in the air
        (if (< (.z (Variables|/Script/Engine.MovementComponent|GetVelocity (Variables|Character|GetCharacterMovement))) 0.0)
          ;[1 1 1] Ledge Collision Line Trace
          (bind (_outhit _returnvalue_7) (Collision|LineTraceByChannel _returnvalue_5 (- _returnvalue_5 "0.000000,0.000000,50.000000") "TraceTypeQuery3" false 0 "None"))
          (if _returnvalue_7
            (bind (_outhit_2 _returnvalue_8) (Collision|LineTraceByChannel (Math|Vector|MakeVector (.x _returnvalue_3) (.y _returnvalue_3) (.Z (Math|Vector|BreakVector (- (.Location (Collision|BreakHitResult _outhit)) "0.000000,0.000000,10.000000")))) (- (.Location (Collision|BreakHitResult _outhit)) "0.000000,0.000000,10.000000") "TraceTypeQuery3" false 0 "None"))
            (if _returnvalue_8
              (Transformation|SetActorLocationAndRotation (+ (+ (.Location (Collision|BreakHitResult _outhit_2)) (* (.ImpactNormal (Collision|BreakHitResult _outhit_2)) 3e+01)) "0.000000,0.000000,20.000000") (Math|Conversions|RotationFromXVector (* (.ImpactNormal (Collision|BreakHitResult _outhit_2)) -1.0)))
              (Variables|Default|SetTemporaryGravity (Variables|/Script/Engine.CharacterMovementComponent|GetGravityScale _charactermovement))
              (Variables|/Script/Engine.CharacterMovementComponent|SetGravityScale _charactermovement 0.0)
              (Components|Movement|StopMovementImmediately _charactermovement)
              (Variables|Default|SetbCanMove false))))))))

(event EventBeginPlay
  ;[1 1 1] Display Player HUD
  (bind _returnvalue (UserInterface|CreateWidget "/Game/GIAMSystem/WidgetBPs/WBP_Player.WBP_Player_C" (Game|GetPlayerController 0)))
  (UserInterface|Viewport|AddtoViewport _returnvalue 0)
  ;[1 1 1] Respawn location for checkpoints
  (Variables|Default|SetRespawnLocation (Math|Transform|MakeTransform (.Location (Math|Transform|BreakTransform (Transformation|GetWorldTransform (Variables|Character|GetMesh))))))
  ;[1 1 1] Load the game, load in the coins
  (bind _returnvalue_2 (SaveGame|LoadGamefromSlot "1"))
  (bind _asbpsg_game_save (Utilities|Casting|CastToBPSG_GameSave _returnvalue_2))
  (Variables|Default|SetCoins (Variables|/Game/GIAMSystem/BPSG_GameSave.BPSG_GameSave_C|GetPlayerCoins _asbpsg_game_save))
  ;[1 1 1] Interaction
  (CallFunction|SetupInteractionTrace))

(event Input|MouseEvents|MouseWheelAxis
  (params (AxisValue :type Float%20%28single-precision%29))
  ;[1 1 1] Scroll wheel to adjust the camera distance, middle mouse button to reset it to default
  (Variables|/Script/Engine.SpringArmComponent|SetTargetArmLength (Variables|Default|GetCameraBoom) (Math|Float|Clamp(Float) (+ (Variables|/Script/Engine.SpringArmComponent|GetTargetArmLength (Variables|Default|GetCameraBoom)) (* AxisValue -1e+01)) 3e+02 1e+03)))

(event Input|KeyboardEvents|R
  (params (Key :type Key%20Structure :default "None"))
  ;[1 1 1] Restart from checkpoint
  (:Pressed
    (Actor|DestroyActor)
    (bind _returnvalue (Game|SpawnActorfromClass "BP_GIAMCharacter_C" (Variables|Default|GetRespawnLocation) "Undefined" "MultiplyWithRoot" 0 0))
    (Pawn|Possess (Game|GetPlayerController 0) _returnvalue)))

(event Input|KeyboardEvents|SpaceBar
  (params (Key :type Key%20Structure :default "None"))
  (bind _returnvalue (Transformation|GetActorLocation))
  ;[1 1 1] Double Jump effect and sound
  (:Pressed
    (if (== (Variables|Default|GetJumpCurrentCount) 1)
      (Effects|SpawnEmitterAttached "/Game/StarterContent/Particles/P_Explosion.P_Explosion" (Variables|Default|GetJumpEffect) "None")
      (Audio|PlaySoundatLocation "/Game/Assets/Ultimate_Platformer_Asset_Pack/Bonus_SFX_Pack/jump-sound-5.jump-sound-5" _returnvalue "0, 0, 0" 1.0 1.0 0.0 0 0 0 0)
      (else
        (Audio|PlaySoundatLocation "/Game/Assets/Ultimate_Platformer_Asset_Pack/Bonus_SFX_Pack/jump-sound-4.jump-sound-4" _returnvalue "0, 0, 0" 1.0 1.0 0.0 0 0 0 0)))))

(event Input|MouseEvents|MiddleMouseButton
  (params (Key :type Key%20Structure :default "None"))
  ;[1 1 1] Scroll wheel to adjust the camera distance, middle mouse button to reset it to default
  (:Pressed
    (Variables|/Script/Engine.SpringArmComponent|SetTargetArmLength (Variables|Default|GetCameraBoom) 4.5e+02)))

(fn ConstructionScript)

(fn SetupInteractionTrace
  (if (Pawn|IsLocallyControlled)
    (Components|Tick|SetComponentTickEnabled (Variables|Default|GetAC_InteractionTrace) true)))